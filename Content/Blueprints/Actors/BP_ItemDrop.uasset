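; BP_ItemDrop is an item drop actor that shrinks away and destroys itself once a BP_PawnTank overlaps it.
; The overlap sets a CanShrink flag, which Tick checks to subtract ScaleReduction uniformly from the actor's scale each frame, independent of delta time.
; The actor is destroyed when its scale is nearly zero, and the file applies no pickup effect to the tank.
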(event `self.ReceiveActorBeginOverlap`
  (params (OtherActor :type "Actor Object Reference"))
  (cast `/Game/Blueprints/Pawns/BP_PawnTank` OtherActor)
  (set `self.bCanShrink` true))

(event `self.ReceiveTick`
  (params (DeltaSeconds :type "Float (single-precision)"))
  (bind (_returnvalue_location _returnvalue_rotation _returnvalue_scale) (`KismetMathLibrary.BreakTransform` (`self.GetTransform`)))
  (bind _scalereduction (`self.ScaleReduction`))
  (if (`self.bCanShrink`)
    (`self.K2_SetActorTransform` (`KismetMathLibrary.MakeTransform` _returnvalue_location _returnvalue_rotation (- _returnvalue_scale (`KismetMathLibrary.MakeVector` _scalereduction _scalereduction _scalereduction))))
    (if (== _returnvalue_scale (0.0 0.0 0.0) :`ErrorTolerance` 0.1)
      (`self.K2_DestroyActor`))))

(fn `UserConstructionScript`)