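; BP_HealthDrop is a health pickup actor that heals the player tank by a fixed amount.
; The OverlappedPlayer event receives the PlayerTank and calls Heal on it, with no destroy step in that path.
; Disconnected leftover nodes would set a shrink flag after a BP_PawnTank cast, scale the actor down and destroy it near zero, but they never run.
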(event `self.ReceiveTick`
  (params (DeltaSeconds :type "Float (single-precision)")))

(event `self.OverlappedPlayer`
  (params (PlayerTank :type "TTPawnTank Object Reference"))
  (`TTPawnBase.Heal` PlayerTank 20.0))

(fn `UserConstructionScript`)