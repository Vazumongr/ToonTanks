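; Player controller that displays a custom mouse cursor through the WBP_MouseCursor widget.
; On BeginPlay it creates the widget, adds it to the viewport at a raised Z-order and sets input mode to game only.
; Every tick it moves the widget to the viewport mouse position, offset by half its desired size so it stays centered on the pointer.
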(event `self.ReceiveBeginPlay`
  (bind _returnvalue (`|CreateWidget` "/Game/Widgets/WBP_MouseCursor.WBP_MouseCursor_C"))
  (set `self.MouseCursorWidget` _returnvalue)
  (`UserWidget.AddToViewport` _returnvalue 50)
  (`WidgetBlueprintLibrary.SetInputMode_GameOnly` self))

(event `self.ReceiveTick`
  (params (DeltaSeconds :type "Float (single-precision)"))
  (bind _returnvalue (`WidgetLayoutLibrary.GetMousePositionOnViewport`))
  (`UserWidget.SetPositionInViewport` (stale `self.ReceiveBeginPlay` _returnvalue) (- _returnvalue (/ (`Widget.GetDesiredSize` (stale `self.ReceiveBeginPlay` _returnvalue)) 2.0)) false))

(fn `UserConstructionScript`)